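; BP_GoStraight is a box the player steps onto and sends sliding in a straight line until blocked.
; An overlap on its top arms a Tick check that turns the character's DirectionIndex into a Direction and swaps the material.
; A looping timer traces ahead, driving Timeline movement, and re-arms direction choice on a hit.
; Stepping off destroys it unless the character's CanRestart is set; Restart restores position and material.
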(event OnComponentEndOverlap(UpBoxComponent)
  (params (OverlappedComponent :type Primitive%20Component%20Object%20Reference) (OtherActor :type Actor%20Object%20Reference) (OtherComp :type Primitive%20Component%20Object%20Reference) (OtherBodyIndex :type Integer))
  (if (Actor|ActorHasTag OtherActor "Player")
    (CallFunction|GetPlayer OtherActor)
    (if (not (Variables|/Script/GJ2024.GJCharacter|GetbCanRestart (Variables|Default|GetAs%20BP%20GJCharacter)))
      (Actor|DestroyActor))))

(event OnComponentBeginOverlap(UpBoxComponent)
  (params (OverlappedComponent :type Primitive%20Component%20Object%20Reference) (OtherActor :type Actor%20Object%20Reference) (OtherComp :type Primitive%20Component%20Object%20Reference) (OtherBodyIndex :type Integer) (bFromSweep :type Boolean) (SweepResult :type Hit%20Result%20Structure%20%28by%20ref%29))
  (if (Actor|ActorHasTag OtherActor "Player")
    (CallFunction|GetPlayer OtherActor)
    (Variables|Default|SetIsCheck true)
    (Variables|/Script/GJ2024.GJCharacter|SetbIsAutoMoving (Variables|Default|GetAs%20BP%20GJCharacter) true)))

(event Custom|ActorDirection
  (bind _as_bp_gjcharacter (Variables|Default|GetAs%20BP%20GJCharacter))
  (bind _as_bp_gjcharacter_2 (Variables|Default|GetAs%20BP%20GJCharacter))
  (bind _as_bp_gjcharacter_3 (Variables|Default|GetAs%20BP%20GJCharacter))
  (bind _as_bp_gjcharacter_4 (Variables|Default|GetAs%20BP%20GJCharacter))
  (if (Variables|Default|GetIsCheck)
    (switch int (Variables|/Script/GJ2024.GJCharacter|GetDirectionIndex (Variables|Default|GetAs%20BP%20GJCharacter))
      (:1
        (bind _returnvalue (Class|GJCharacter|CalculateDirectiontoAngle _as_bp_gjcharacter_3 (Transformation|GetActorForwardVector _as_bp_gjcharacter_3)))
        (Variables|Default|SetDirection _returnvalue))
      (:2
        (bind _returnvalue_2 (Class|GJCharacter|CalculateDirectiontoAngle _as_bp_gjcharacter (Transformation|GetActorRightVector _as_bp_gjcharacter)))
        (Variables|Default|SetDirection _returnvalue_2))
      (:3
        (bind _returnvalue_3 (Class|GJCharacter|CalculateDirectiontoAngle _as_bp_gjcharacter_2 (* (Transformation|GetActorRightVector _as_bp_gjcharacter_2) -1.0)))
        (Variables|Default|SetDirection _returnvalue_3))
      (:4
        (bind _returnvalue_4 (Class|GJCharacter|CalculateDirectiontoAngle _as_bp_gjcharacter_4 (* (Transformation|GetActorForwardVector _as_bp_gjcharacter_4) -1.0)))
        (Variables|Default|SetDirection _returnvalue_4)))
    (Variables|/Script/GJ2024.GJCharacter|SetDirectionIndex (Variables|Default|GetAs%20BP%20GJCharacter) 0)
    (Variables|Default|SetIsCheck false)
    (bind _returnvalue_5 (Utilities|Time|SetTimerbyFunctionName 0 "ActorMove" 0.1 true))
    (Variables|Default|SetActorMoveTimerHandle _returnvalue_5)
    (Rendering|Material|SetMaterial (Variables|Default|GetBoxMesh) 0 "/Engine/VREditor/BasicMeshes/MI_Cube_01.MI_Cube_01")))

(event Custom|ActorMove
  (bind _returnvalue (Transformation|GetActorLocation))
  (bind _direction (Variables|Default|GetDirection))
  (bind _outhit (Collision|LineTraceForObjects (+ (* _direction (* (Variables|Default|GetBound) 1.05)) _returnvalue) (+ _returnvalue (* _direction (* (Variables|Default|GetBound) 1.2))) (Variables|Default|GetObject%20Types) false 0 "None"))
  (if (.bBlockingHit (Collision|BreakHitResult _outhit))
    (Utilities|Time|ClearandInvalidateTimerbyHandle (Variables|Default|GetActorMoveTimerHandle))
    (Variables|Default|SetIsCheck true)
    (else
      (Timeline|时间轴 Play
        (:Update
          (if (.bBlockingHit (Collision|BreakHitResult _outhit))
            (Timeline|时间轴 Stop)
            (elif (Variables|/Script/GJ2024.GJCharacter|GetbIsAutoMoving (Variables|Default|GetAs%20BP%20GJCharacter))
              (Transformation|SetActorLocation (+ (* (Variables|Default|GetDirection) 5.0) (Transformation|GetActorLocation)) false false))))
        (:Finished
          (Timeline|时间轴 PlayFromStart))))))

(event EventBeginPlay
  (Variables|Default|SetBound (Math|Conversions|ToFloat(Integer) (Math|Float|Ceil (.x (.BoxExtent (Collision|GetComponentBounds (Variables|Default|GetBoxMesh)))))))
  (Variables|Default|SetStartLocation (Transformation|GetActorLocation))
  (Variables|Default|SetOriginalMaterial (Rendering|Material|GetMaterial (Variables|Default|GetBoxMesh) 0)))

(event Collision|EventActorBeginOverlap
  (params (OtherActor :type Actor%20Object%20Reference)))

(event EventTick
  (params (DeltaSeconds :type Float%20%28single-precision%29))
  (CallFunction|ActorDirection))

(event EventRestart
  (Variables|Default|SetIsCheck false)
  (Utilities|Time|ClearandInvalidateTimerbyHandle (Variables|Default|GetActorMoveTimerHandle))
  (Utilities|FlowControl|Delay 0.05)
  (Transformation|SetActorLocation (Variables|Default|GetStartLocation) false false)
  (Rendering|Material|SetMaterial (Variables|Default|GetBoxMesh) 0 (Variables|Default|GetOriginalMaterial)))

(fn ConstructionScript)

(fn GetPlayer
  (params (Object :type Actor%20Object%20Reference))
  (Utilities|IsValid (Variables|Default|GetAs%20BP%20GJCharacter)
    (:Is%20Not%20Valid
      (bind _asbp_gjcharacter (Utilities|Casting|CastToBP_GJCharacter Object))
      (Variables|Default|SetAs%20BP%20GJCharacter _asbp_gjcharacter))))