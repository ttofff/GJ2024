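; BP_BoxTeleport is a trigger-box actor that teleports the player character to an offset from the box's own location.
; Overlap by an actor tagged Player caches the BP_GJCharacter, disables input and plays the Move timeline to animate its scale.
; When that finishes, the character is relocated and the Big timeline animates scale again.
; Input is then restored, and the box destroys itself if IsDestroy is set.
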(event OnComponentBeginOverlap(BoxComponent)
  (params (OverlappedComponent :type Primitive%20Component%20Object%20Reference) (OtherActor :type Actor%20Object%20Reference) (OtherComp :type Primitive%20Component%20Object%20Reference) (OtherBodyIndex :type Integer) (bFromSweep :type Boolean) (SweepResult :type Hit%20Result%20Structure%20%28by%20ref%29))
  (bind _as_bp_gjcharacter (Variables|Default|GetAs%20BP%20GJCharacter))
  (bind _as_bp_gjcharacter_2 (Variables|Default|GetAs%20BP%20GJCharacter))
  (if (Actor|ActorHasTag OtherActor "Player")
    (CallFunction|GetPlayer OtherActor)
    ;[1 1 1] 传送
    (Development|PrintString "Teleport")
    (Input|DisableInput (Variables|Default|GetAs%20BP%20GJCharacter) (Game|GetPlayerController 0))
    (bind _新建轨道_0 (Timeline|Move PlayFromStart)
      (:Update
        (Transformation|SetActorScale3D _as_bp_gjcharacter_2 (Math|Vector|MakeVector _新建轨道_0 _新建轨道_0 _新建轨道_0)))
      (:Finished
        (Transformation|SetActorLocation _as_bp_gjcharacter_2 (+ (Variables|Default|GetTeleportLocation) (Transformation|GetActorLocation)) false false)
        (bind _新建轨道_0_2 (Timeline|Big PlayFromStart)
          (:Update
            (Transformation|SetActorScale3D _as_bp_gjcharacter (Math|Vector|MakeVector _新建轨道_0_2 _新建轨道_0_2 _新建轨道_0_2)))
          (:Finished
            (Input|EnableInput _as_bp_gjcharacter (Game|GetPlayerController 0))
            (if (Variables|Default|GetIsDestroy)
              (Actor|DestroyActor))))))))

(event EventBeginPlay)

(event Collision|EventActorBeginOverlap
  (params (OtherActor :type Actor%20Object%20Reference)))

(event EventTick
  (params (DeltaSeconds :type Float%20%28single-precision%29)))

(fn ConstructionScript)

(fn GetPlayer
  (params (Object :type Actor%20Object%20Reference))
  (Utilities|IsValid (Variables|Default|GetAs%20BP%20GJCharacter)
    (:Is%20Not%20Valid
      (bind _asbp_gjcharacter (Utilities|Casting|CastToBP_GJCharacter Object))
      (Variables|Default|SetAs%20BP%20GJCharacter _asbp_gjcharacter))))