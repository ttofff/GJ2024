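; BP_OneStroke is a tile for a one-stroke path puzzle, where the player steps on tiles that cannot be re-entered.
; Stepping changes the tile's material and marks it stepped; leaving makes it block pawns.
; The end tile starts a recursive check through four-direction line traces, and any tile finding an unstepped neighbor calls the character's SetRestartLocation.
; Restart restores the tile's flags, collision and original material.
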(event OnComponentBeginOverlap(UpBoxComponent)
  (params (OverlappedComponent :type Primitive%20Component%20Object%20Reference) (OtherActor :type Actor%20Object%20Reference) (OtherComp :type Primitive%20Component%20Object%20Reference) (OtherBodyIndex :type Integer) (bFromSweep :type Boolean) (SweepResult :type Hit%20Result%20Structure%20%28by%20ref%29))
  (bind _boxmesh (Variables|Default|GetBoxMesh))
  (if (Actor|ActorHasTag OtherActor "Player")
    (CallFunction|GetPlayer OtherActor)
    (Development|PrintString "Step")
    (Variables|Default|SetbIsStepped true)
    (Variables|Default|SetOriginalMaterial (Rendering|Material|GetMaterial _boxmesh 0))
    (Rendering|Material|SetMaterial _boxmesh 0 "/Engine/VREditor/BasicMeshes/MI_Cube_03.MI_Cube_03")
    (if (Variables|Default|GetIsEnd)
      (CallFunction|CheckStep))))

(event OnComponentEndOverlap(BlockBoxComponent)
  (params (OverlappedComponent :type Primitive%20Component%20Object%20Reference) (OtherActor :type Actor%20Object%20Reference) (OtherComp :type Primitive%20Component%20Object%20Reference) (OtherBodyIndex :type Integer))
  (bind _blockboxcomponent (Variables|Default|GetBlockBoxComponent))
  (if (Actor|ActorHasTag OtherActor "Player")
    (Collision|SetCollisionEnabled _blockboxcomponent "QueryAndPhysics")
    (Collision|SetCollisionResponsetoChannel _blockboxcomponent "ECC_Pawn" "ECR_Block")
    (Collision|SetCollisionEnabled (Variables|Default|GetUpBoxComponent) "NoCollision")))

(event Custom|CheckStep
  (bind _returnvalue (Transformation|GetActorLocation))
  (for _array_element (Variables|Default|GetDirection)
    (bind _outhit (Collision|LineTraceForObjects (+ (* _array_element (+ (Variables|Default|GetBound) 1e+01)) _returnvalue) (+ _returnvalue (* _array_element (* (Variables|Default|GetBound) 2.0))) (Variables|Default|GetObject%20Types) false 0 "None"))
    (if (.bBlockingHit (Collision|BreakHitResult _outhit))
      (bind _asbp_one_stroke (Utilities|Casting|CastToBP_OneStroke (.HitActor (Collision|BreakHitResult _outhit))))
      (if (and (Variables|/Script/GJ2024.OneStroke|GetbIsStepped _asbp_one_stroke) (not (Variables|Default|GetIsFlag)))
        (if (not (Variables|/Script/GJ2024.OneStroke|GetbIsCheck _asbp_one_stroke))
          (Variables|/Script/GJ2024.OneStroke|SetbIsCheck _asbp_one_stroke true)
          (CallFunction|CheckStep _asbp_one_stroke))
        (else
          (Variables|Default|SetIsFlag true)))))
  (Variables|Default|SetbIsCheck true)
  (if (Variables|Default|GetIsFlag)
    (Default|SetRestartLocation (Variables|Default|GetAs%20BP%20GJCharacter))))

(event EventBeginPlay
  (Variables|Default|SetBound (Math|Conversions|ToFloat(Integer) (Math|Float|Ceil (.x (.BoxExtent (Collision|GetComponentBounds (Variables|Default|GetBoxMesh)))))))
  (Utilities|Array|Add (Variables|Default|GetDirection) (Transformation|GetActorForwardVector))
  (Utilities|Array|Add (Variables|Default|GetDirection) (* (Transformation|GetActorForwardVector) -1.0))
  (Utilities|Array|Add (Variables|Default|GetDirection) (Transformation|GetActorRightVector))
  (Utilities|Array|Add (Variables|Default|GetDirection) (* (Transformation|GetActorRightVector) -1.0)))

(event Collision|EventActorBeginOverlap
  (params (OtherActor :type Actor%20Object%20Reference)))

(event EventTick
  (params (DeltaSeconds :type Float%20%28single-precision%29)))

(event EventRestart
  (bind _blockboxcomponent (Variables|Default|GetBlockBoxComponent))
  (Variables|Default|SetbIsStepped false)
  (Variables|Default|SetbIsCheck false)
  (Variables|Default|SetIsFlag false)
  (Collision|SetCollisionEnabled _blockboxcomponent "QueryOnly")
  (Collision|SetCollisionResponsetoChannel _blockboxcomponent "ECC_Pawn" "ECR_Overlap")
  (Collision|SetCollisionEnabled (Variables|Default|GetUpBoxComponent) "QueryOnly")
  (Rendering|Material|SetMaterial (Variables|Default|GetBoxMesh) 0 (Variables|Default|GetOriginalMaterial)))

(fn ConstructionScript)

(fn GetPlayer
  (params (Object :type Actor%20Object%20Reference))
  (Utilities|IsValid (Variables|Default|GetAs%20BP%20GJCharacter)
    (:Is%20Not%20Valid
      (bind _asbp_gjcharacter (Utilities|Casting|CastToBP_GJCharacter Object))
      (Variables|Default|SetAs%20BP%20GJCharacter _asbp_gjcharacter))))