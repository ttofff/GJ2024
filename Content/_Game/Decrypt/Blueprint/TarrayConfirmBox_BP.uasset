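; TarrayConfirmBox_BP is a puzzle checker that counts how many confirm boxes within its Box volume hold a box.
; BeginPlay starts an endless 0.1-second loop that toggles the volume's collision on and off to re-fire begin-overlap events.
; Each overlap with a tagged BP_ConfirmBox compares IsHaveBox against IsCheck to raise or lower Num.
; An increment that brings Num to SuccessNum only prints a message.
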(event OnComponentBeginOverlap(Box)
  (params (OverlappedComponent :type Primitive%20Component%20Object%20Reference) (OtherActor :type Actor%20Object%20Reference) (OtherComp :type Primitive%20Component%20Object%20Reference) (OtherBodyIndex :type Integer) (bFromSweep :type Boolean) (SweepResult :type Hit%20Result%20Structure%20%28by%20ref%29))
  (if (Actor|ActorHasTag OtherActor "ConfirmBox")
    (bind _asbp_confirm_box (Utilities|Casting|CastToBP_ConfirmBox OtherActor))
    (if (and (Variables|/Script/GJ2024.ConfirmBox|GetbIsHaveBox _asbp_confirm_box) (not (Variables|/Game/_Game/Decrypt/Blueprint/BP_ConfirmBox.BP_ConfirmBox_C|GetIsCheck _asbp_confirm_box)))
      (Math|Integer|IncrementInt (Variables|Default|GetNum)
        (:%20%20
          (Variables|/Game/_Game/Decrypt/Blueprint/BP_ConfirmBox.BP_ConfirmBox_C|SetIsCheck _asbp_confirm_box true)
          (if (>= (Variables|Default|GetNum) (Variables|Default|GetSuccessNum))
            (Development|PrintString "Hello" true true "(R=1.000000,G=0.491760,B=0.737550,A=1.000000)"))))
      (elif (Variables|/Game/_Game/Decrypt/Blueprint/BP_ConfirmBox.BP_ConfirmBox_C|GetIsCheck _asbp_confirm_box)
        (Math|Integer|DecrementInt (Variables|Default|GetNum)
          (:%20%20
            (Variables|/Game/_Game/Decrypt/Blueprint/BP_ConfirmBox.BP_ConfirmBox_C|SetIsCheck _asbp_confirm_box false)))))))

(event EventBeginPlay
  (Collision|SetCollisionEnabled (Variables|Default|GetBox) "QueryOnly" :!label _label)
  (Collision|SetCollisionEnabled (Variables|Default|GetBox) "NoCollision")
  (Utilities|FlowControl|Delay 0.1)
  (goto _label))

(event Collision|EventActorBeginOverlap
  (params (OtherActor :type Actor%20Object%20Reference)))

(event EventTick
  (params (DeltaSeconds :type Float%20%28single-precision%29)))

(fn ConstructionScript)