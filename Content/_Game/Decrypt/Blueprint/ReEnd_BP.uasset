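; ReEnd_BP is a one-shot trigger actor in the Decrypt folder that appears to mark an end point for the player.
; When a Player-tagged actor overlaps its Box, GetPlayer caches the BP_GJCharacter, then the trigger disables restart, stops auto-movement and resets the direction index.
; It removes both static meshes, spawns an actor of the Class variable at the Scene transform, and destroys itself after a short delay.
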(event OnComponentBeginOverlap(Box)
  (params (OverlappedComponent :type Primitive%20Component%20Object%20Reference) (OtherActor :type Actor%20Object%20Reference) (OtherComp :type Primitive%20Component%20Object%20Reference) (OtherBodyIndex :type Integer) (bFromSweep :type Boolean) (SweepResult :type Hit%20Result%20Structure%20%28by%20ref%29))
  (bind _as_bp_gjcharacter (Variables|Default|GetAs%20BP%20GJCharacter))
  (if (Actor|ActorHasTag OtherActor "Player")
    (CallFunction|GetPlayer OtherActor)
    (Variables|/Script/GJ2024.GJCharacter|SetbCanRestart _as_bp_gjcharacter false)
    (Variables|/Script/GJ2024.GJCharacter|SetbIsAutoMoving _as_bp_gjcharacter false)
    (Variables|/Script/GJ2024.GJCharacter|SetDirectionIndex _as_bp_gjcharacter 0)
    (Components|DestroyComponent (Variables|Default|GetStaticMesh))
    (Game|SpawnActorfromClass (Variables|Default|GetClass) (Transformation|GetWorldTransform (Variables|Default|GetScene)) "Undefined" "MultiplyWithRoot" 0 0)
    (Utilities|FlowControl|Delay 0.2)
    (Actor|DestroyActor)))

(event EventBeginPlay)

(event Collision|EventActorBeginOverlap
  (params (OtherActor :type Actor%20Object%20Reference)))

(event EventTick
  (params (DeltaSeconds :type Float%20%28single-precision%29)))

(fn ConstructionScript)

(fn GetPlayer
  (params (Object :type Actor%20Object%20Reference))
  (Utilities|IsValid (Variables|Default|GetAs%20BP%20GJCharacter)
    (:Is%20Not%20Valid
      (bind _asbp_gjcharacter (Utilities|Casting|CastToBP_GJCharacter Object))
      (Variables|Default|SetAs%20BP%20GJCharacter _asbp_gjcharacter))))