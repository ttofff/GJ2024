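; BP_PushBox is a pushable box that slides one box-width when a tagged Interactive component of the player overlaps one of its four side triggers.
; The trigger's forward vector sets the direction, opposite to travel, and a line trace cancels the push if blocked.
; A looping timer runs MoveBox to step the box, with triggers disabled until the distance to target starts growing.
; Restart returns the box to its starting location.
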(event OnComponentBeginOverlap(ForwardBoxComponent)
  (params (OverlappedComponent :type Primitive%20Component%20Object%20Reference) (OtherActor :type Actor%20Object%20Reference) (OtherComp :type Primitive%20Component%20Object%20Reference) (OtherBodyIndex :type Integer) (bFromSweep :type Boolean) (SweepResult :type Hit%20Result%20Structure%20%28by%20ref%29))
  (CallFunction|PushDirection OtherActor OtherComp (Variables|Default|GetForwardBoxComponent)))

(event OnComponentBeginOverlap(BackBoxComponent)
  (params (OverlappedComponent :type Primitive%20Component%20Object%20Reference) (OtherActor :type Actor%20Object%20Reference) (OtherComp :type Primitive%20Component%20Object%20Reference) (OtherBodyIndex :type Integer) (bFromSweep :type Boolean) (SweepResult :type Hit%20Result%20Structure%20%28by%20ref%29))
  (CallFunction|PushDirection OtherActor OtherComp (Variables|Default|GetBackBoxComponent)))

(event OnComponentBeginOverlap(RightBoxComponent)
  (params (OverlappedComponent :type Primitive%20Component%20Object%20Reference) (OtherActor :type Actor%20Object%20Reference) (OtherComp :type Primitive%20Component%20Object%20Reference) (OtherBodyIndex :type Integer) (bFromSweep :type Boolean) (SweepResult :type Hit%20Result%20Structure%20%28by%20ref%29))
  (CallFunction|PushDirection OtherActor OtherComp (Variables|Default|GetRightBoxComponent)))

(event OnComponentBeginOverlap(LeftBoxComponent)
  (params (OverlappedComponent :type Primitive%20Component%20Object%20Reference) (OtherActor :type Actor%20Object%20Reference) (OtherComp :type Primitive%20Component%20Object%20Reference) (OtherBodyIndex :type Integer) (bFromSweep :type Boolean) (SweepResult :type Hit%20Result%20Structure%20%28by%20ref%29))
  (CallFunction|PushDirection OtherActor OtherComp (Variables|Default|GetLeftBoxComponent)))

(event Custom|MoveBox
  (bind _returnvalue (Transformation|GetActorLocation))
  (bind _directionlocation (Variables|Default|GetDirectionLocation))
  (bind _actorlocation (Variables|Default|GetActorLocation))
  (bind _bound (Variables|Default|GetBound))
  (bind _bound_2 (Variables|Default|GetBound))
  (bind _returnvalue_2 (* _bound -1.0))
  (bind _returnvalue_3 (/ _bound_2 -5e+01))
  (bind _returnvalue_4 (* _directionlocation _returnvalue_2))
  (bind _returnvalue_5 (* _directionlocation _returnvalue_3))
  (bind _returnvalue_6 (+ _returnvalue_4 _actorlocation))
  (bind _returnvalue_7 (+ _returnvalue_5 _returnvalue))
  (bind _returnvalue_8 (Math|Vector|Distance(Vector) _returnvalue_6 _returnvalue_7))
  (if (< (Variables|Default|GetLastDistance) _returnvalue_8)
    (Collision|SetCollisionEnabled (Variables|Default|GetForwardBoxComponent) "QueryOnly")
    (Utilities|Time|ClearandInvalidateTimerbyHandle (Variables|Default|GetMoveTimerHandle))
    (else
      (Variables|Default|SetLastDistance _returnvalue_8)
      (Transformation|SetActorLocation _returnvalue_7 false false))))

(event EventBeginPlay
  (Variables|Default|SetStartLocation (Transformation|GetActorLocation))
  (Variables|Default|SetBound (Math|Conversions|ToFloat(Integer) (* (Math|Float|Ceil (.x (.BoxExtent (Collision|GetComponentBounds (Variables|Default|GetBoxMesh))))) 2))))

(event Collision|EventActorBeginOverlap
  (params (OtherActor :type Actor%20Object%20Reference)))

(event EventTick
  (params (DeltaSeconds :type Float%20%28single-precision%29)))

(event EventRestart
  (Transformation|SetActorLocation (Variables|Default|GetStartLocation) false false))

(fn ConstructionScript)

(fn GetPlayer
  (params (Object :type Actor%20Object%20Reference))
  (Utilities|IsValid (Variables|Default|GetAs%20BP%20GJCharacter)
    (:Is%20Not%20Valid
      (bind _asbp_gjcharacter (Utilities|Casting|CastToBP_GJCharacter Object))
      (Variables|Default|SetAs%20BP%20GJCharacter _asbp_gjcharacter))))

(fn PushDirection
  (params (Actor :type Actor%20Object%20Reference) (Comp :type Actor%20Component%20Object%20Reference) (BoxActor :type Box%20Component%20Object%20Reference))
  (bind _returnvalue (Math|Vector|GetForwardVector BoxActor))
  (bind _returnvalue_2 (Transformation|GetActorLocation))
  (bind _bound (Variables|Default|GetBound))
  (bind _returnvalue_3 (* _bound -1.0))
  (if (and (Actor|ActorHasTag Actor "Player") (Components|ComponentHasTag Comp "Interactive"))
    (CallFunction|GetPlayer Actor)
    (Variables|Default|SetDirectionLocation _returnvalue)
    (bind _outhit (Collision|LineTraceForObjects (+ _returnvalue_2 (* _returnvalue (- (/ _returnvalue_3 2.0) 1e+01))) (+ (* _returnvalue _returnvalue_3) _returnvalue_2) (Variables|Default|GetObject%20Types) false 0 "ForDuration"))
    (if (not (.bBlockingHit (Collision|BreakHitResult _outhit)))
      (Collision|SetCollisionEnabled (Variables|Default|GetForwardBoxComponent) "NoCollision")
      (Variables|Default|SetActorLocation (Transformation|GetActorLocation))
      (Variables|Default|SetLastDistance 4e+02)
      (bind _returnvalue_4 (Utilities|Time|SetTimerbyFunctionName 0 "MoveBox" 0.01 true))
      (Variables|Default|SetMoveTimerHandle _returnvalue_4))))