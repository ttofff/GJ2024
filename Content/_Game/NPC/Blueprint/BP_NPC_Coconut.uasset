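; BP_NPC_Coconut is a coconut NPC that talks to the player, grants the coconut transformation (faster running), then relocates to camp.
; Overlap by the player's Interactive-tagged component steps through scripted lines in a widget, cleared by timer.
; After the last line it unlocks the character's mesh entry, shows a notification and teleports behind a Niagara cloud.
; Thereafter it shows common lines with randomized indices; a separate trigger reveals the initial tip.
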(event OnComponentBeginOverlap(InteractionCollision)
  (params (OverlappedComponent :type Primitive%20Component%20Object%20Reference) (OtherActor :type Actor%20Object%20Reference) (OtherComp :type Primitive%20Component%20Object%20Reference) (OtherBodyIndex :type Integer) (bFromSweep :type Boolean) (SweepResult :type Hit%20Result%20Structure%20%28by%20ref%29))
  (if (and (Actor|ActorHasTag OtherActor "Player") (Components|ComponentHasTag OtherComp "Interactive"))
    (CallFunction|GetPlayer OtherActor)
    (Rendering|SetVisibility (Variables|Default|GetTip) false false)
    (Collision|SetCollisionEnabled (Variables|Default|GetTipCollision) "NoCollision")
    (Variables|Default|SetbIsClick true)
    (Utilities|Time|ClearandInvalidateTimerbyHandle (Variables|Default|GetDisappearTimerHandle))
    (bind _asui_text (Utilities|Casting|CastToUI_Text (UserInterface|GetUserWidgetObject (Variables|Default|GetWidget))))
    (if (Variables|Default|GetbIsCommon)
      (Variables|/Game/_Game/NPC/UMG/UI_Text.UI_Text_C|SetTextContent _asui_text (Utilities|Array|Get(acopy) (Variables|Default|GetCommonTexts) (Variables|Default|GetIndexText)))
      (Variables|Default|SetIndexText (Math|Random|RandomIntegerinRange 0 1))
      (bind _returnvalue (Utilities|Time|SetTimerbyFunctionName 0 "Clear" 2.0))
      (Variables|Default|SetDisappearTimerHandle _returnvalue)
      (else
        (Variables|/Game/_Game/NPC/UMG/UI_Text.UI_Text_C|SetTextContent _asui_text (Utilities|Array|Get(acopy) (Variables|Default|GetInteractionTexts) (Variables|Default|GetIndexText)))
        (Math|Integer|IncrementInt (Variables|Default|GetIndexText)
          (:%20%20
            (bind _returnvalue_2 (Utilities|Time|SetTimerbyFunctionName 0 "Clear" 2.0))
            (Variables|Default|SetDisappearTimerHandle _returnvalue_2)
            (CallFunction|TransferLocation)))))))

(event OnComponentBeginOverlap(TipCollision)
  (params (OverlappedComponent :type Primitive%20Component%20Object%20Reference) (OtherActor :type Actor%20Object%20Reference) (OtherComp :type Primitive%20Component%20Object%20Reference) (OtherBodyIndex :type Integer) (bFromSweep :type Boolean) (SweepResult :type Hit%20Result%20Structure%20%28by%20ref%29))
  (if (Actor|ActorHasTag OtherActor "Player")
    (CallFunction|GetPlayer)
    (Rendering|SetVisibility (Variables|Default|GetTip) true false)))

(event Custom|Clear
  (bind _asui_text (Utilities|Casting|CastToUI_Text (UserInterface|GetUserWidgetObject (Variables|Default|GetWidget))))
  (Variables|/Game/_Game/NPC/UMG/UI_Text.UI_Text_C|SetTextContent _asui_text ""))

(event Custom|TransferLocation
  (if (>= (Variables|Default|GetIndexText) (Utilities|Array|Length (Variables|Default|GetInteractionTexts)))
    (Variables|Default|SetbIsCommon true)
    (Variables|Default|SetIndexText 0)
    (|SetBy-RefVar (.ishave (Utilities|Array|Get(acopy) (Variables|/Game/_Game/_Player/_Blueprint/BP_GJCharacter.BP_GJCharacter_C|GetChangeMeshInfo (Variables|Default|GetAs%20BP%20GJCharacter)) 4)) true)
    (Default|IntoNotifyAnim (Variables|/Game/_Game/_Player/_Blueprint/BP_GJCharacter.BP_GJCharacter_C|GetUI_Player (Variables|Default|GetAs%20BP%20GJCharacter)) "获得椰子的变身，奔跑速度加快，通过R键装备")
    (Collision|SetCollisionEnabled (Variables|Default|GetInteractionCollision) "NoCollision")
    (Utilities|FlowControl|Delay 2.0)
    (bind _returnvalue (Niagara|SpawnSystematLocation "/Game/_Game/Material/NS_Cloud.NS_Cloud" (Transformation|GetWorldLocation (Variables|Default|GetDisappearNiagaraComponent))))
    (Utilities|FlowControl|Delay 0.5)
    (Transformation|SetActorLocation (Variables|Default|GetCampLocation) false false)
    (Utilities|FlowControl|Delay 0.2)
    (Components|Activation|Deactivate _returnvalue)
    (Collision|SetCollisionEnabled (Variables|Default|GetInteractionCollision) "QueryOnly")))

(event EventBeginPlay)

(event Collision|EventActorBeginOverlap
  (params (OtherActor :type Actor%20Object%20Reference)))

(event EventTick
  (params (DeltaSeconds :type Float%20%28single-precision%29)))

(fn ConstructionScript)

(fn GetPlayer
  (params (Object :type Actor%20Object%20Reference))
  (Utilities|IsValid (Variables|Default|GetAs%20BP%20GJCharacter)
    (:Is%20Not%20Valid
      (bind _asbp_gjcharacter (Utilities|Casting|CastToBP_GJCharacter Object))
      (Variables|Default|SetAs%20BP%20GJCharacter _asbp_gjcharacter))))