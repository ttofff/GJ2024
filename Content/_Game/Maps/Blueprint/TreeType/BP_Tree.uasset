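; BP_Tree is a choppable tree that leaves a pickup-style falling object carrying its item info.
; Overlap from a Player-tagged actor's Attack-tagged component calls ChopDownTree, which is defined outside this graph.
; Tick polls the one-shot IsSpawn flag, then traces down from FallingObjectsSceneSpawn.
; On a hit it destroys the trunk mesh and spawns BP_FallingObjects_Tree just above that point, passing TreeItemInfo.
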(event OnComponentBeginOverlap(TreeCollision)
  (params (OverlappedComponent :type Primitive%20Component%20Object%20Reference) (OtherActor :type Actor%20Object%20Reference) (OtherComp :type Primitive%20Component%20Object%20Reference) (OtherBodyIndex :type Integer) (bFromSweep :type Boolean) (SweepResult :type Hit%20Result%20Structure%20%28by%20ref%29))
  (if (and (Actor|ActorHasTag OtherActor "Player") (Components|ComponentHasTag OtherComp "Attack"))
    (Class|Tree|ChopDownTree OtherActor)))

(event Custom|SpawnFallingObjects
  (bind _fallingobjectsscenespawn (Variables|Default|GetFallingObjectsSceneSpawn))
  (bind _returnvalue (Transformation|GetWorldLocation _fallingobjectsscenespawn))
  ;[1 1 1] 生成掉落物
  (if (Variables|Default|GetbIsSpawn)
    (Variables|Default|SetbIsSpawn false)
    (bind _outhit (Collision|LineTraceForObjects _returnvalue (+ _returnvalue "0.000000,0.000000,-300.000000") (Variables|Default|GetObject%20Types) false 0 "None"))
    (if (.bBlockingHit (Collision|BreakHitResult _outhit))
      (Variables|Default|SetLastTrunkLocation (.Location (Collision|BreakHitResult _outhit)))
      (Components|DestroyComponent (Variables|Default|GetTreeTrunkMeshComponent))
      (bind _returnvalue_2 (Game|SpawnActorfromClass "/Game/_Game/Maps/Blueprint/FallingObjectsType/BP_FallingObjects_Tree.BP_FallingObjects_Tree_C" (Math|Transform|MakeTransform (+ (Variables|Default|GetLastTrunkLocation) "0.000000,0.000000,10.000000") "0, 0, 0" "1.000000,1.000000,1.000000") "Undefined" "MultiplyWithRoot" 0 0))
      (Variables|/Script/GJ2024.FallingObjects|SetItemInfo _returnvalue_2 (Variables|Default|GetTreeItemInfo)))))

(event EventBeginPlay)

(event Collision|EventActorBeginOverlap
  (params (OtherActor :type Actor%20Object%20Reference)))

(event EventTick
  (params (DeltaSeconds :type Float%20%28single-precision%29))
  (CallFunction|SpawnFallingObjects))

(fn ConstructionScript)