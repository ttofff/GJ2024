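; BP_FallingObjects is a backpack pickup actor, with extra counters for wood, stone, iron and food.
; On BeginPlay it builds its item info from a data table row keyed by the item class enum.
; A timeline then animates its scale, and a short delay later enables query-only sphere collision.
; Player-tagged overlap adds the item to the character's backpack, increments the matching resource counter and destroys the actor.
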(event OnComponentBeginOverlap(SphereComponent)
  (params (OverlappedComponent :type Primitive%20Component%20Object%20Reference) (OtherActor :type Actor%20Object%20Reference) (OtherComp :type Primitive%20Component%20Object%20Reference) (OtherBodyIndex :type Integer) (bFromSweep :type Boolean) (SweepResult :type Hit%20Result%20Structure%20%28by%20ref%29))
  (bind _as_bp_gjcharacter (Variables|Default|GetAs%20BP%20GJCharacter))
  (bind _backpackinfo (Variables|/Script/GJ2024.GJCharacter|GetBackpackInfo _as_bp_gjcharacter))
  (if (Actor|ActorHasTag OtherActor "Player")
    (CallFunction|GetPlayer OtherActor)
    (Default|BackpackAdd _as_bp_gjcharacter (Variables|Default|GetInfo))
    (switch Utilities|FlowControl|Switch|SwitchonEBackpackClass (Variables|Default|GetItemBackpackClass)
      (:E_Wood
        (Math|Integer|IncrementInt (.woodcnt _backpackinfo)
          (:%20%20
            _)))
      (:E_Stone
        (Math|Integer|IncrementInt (.stonecnt _backpackinfo)
          (:%20%20
            _)))
      (:E_Iron
        (Math|Integer|IncrementInt (.ironcnt _backpackinfo)
          (:%20%20
            _)))
      (:E_Food
        (Math|Integer|IncrementInt (.foodcnt _backpackinfo)
          (:%20%20
            _))))
    (Actor|DestroyActor)))

(event EventBeginPlay
  (bind _returnvalue (Utilities|GetDataTableRow "/Game/_Game/_Player/Backpack/BackpackDataTable.BackpackDataTable" (Utilities|String|StringToName (Utilities|String|EnumtoString (Variables|Default|GetItemBackpackClass))))
    (:then
      (Variables|Default|SetInfo (Utilities|Struct|MakeFBackpackInfo (.name _returnvalue) (.index _returnvalue) (.image _returnvalue) (.isstack _returnvalue) (Variables|Default|GetCnt) (.maxcount _returnvalue) (.class _returnvalue) (.isempty _returnvalue) (.sortnum _returnvalue) (.canuse _returnvalue)))
      (bind _新建轨道_0 (Timeline|时间轴 PlayFromStart)
        (:Update
          (Transformation|SetActorScale3D (Math|Vector|MakeVector _新建轨道_0 _新建轨道_0 _新建轨道_0)))
        (:Finished
          (Utilities|FlowControl|Delay 0.2)
          (Collision|SetCollisionEnabled (Variables|Default|GetSphereComponent) "QueryOnly"))))))

(event Collision|EventActorBeginOverlap
  (params (OtherActor :type Actor%20Object%20Reference)))

(event EventTick
  (params (DeltaSeconds :type Float%20%28single-precision%29)))

(fn ConstructionScript)

(fn GetPlayer
  (params (Object :type Object%20Object%20Reference))
  (Utilities|IsValid (Variables|Default|GetAs%20BP%20GJCharacter)
    (:Is%20Not%20Valid
      (bind _asbp_gjcharacter (Utilities|Casting|CastToBP_GJCharacter Object))
      (Variables|Default|SetAs%20BP%20GJCharacter _asbp_gjcharacter))))