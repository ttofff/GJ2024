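; Player character Blueprint that owns the backpack and shortcut-bar inventory and the player HUD.
; Tick polls one-shot flags to spawn the selected axe, pickaxe or hammer on the Tool socket and to toggle backpack and mesh-change screens, which freeze time dilation.
; Inventory functions stack, reduce, delete with re-indexing, and drag-swap items between backpack and shortcuts, refreshing the widgets.
; An event toggles the workbench UI without pausing.
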(event Custom|OpenWorkbench_UI
  (bind _returnvalue (Game|GetPlayerController 0))
  (bind _ui_player (Variables|Default|GetUI_Player))
  (bind _ui_workbench (Variables|/Game/_Game/UMG/_Player/UI_Player.UI_Player_C|GetUI_Workbench _ui_player))
  ;[1 1 1] 打开工作台UI
  (if (Variables|Default|GetbIsOpenedWorkbench)
    (Variables|Default|SetbIsOpenedWorkbench false)
    (Variables|Default|SetCharacterStates "E_Common")
    (Input|SetInputModeGameOnly (Game|GetPlayerController 0) false)
    (Variables|/Script/Engine.PlayerController|SetbShowMouseCursor (Game|GetPlayerController 0) false)
    (Widget|SetVisibility (Variables|/Game/_Game/UMG/_Player/UI_Player.UI_Player_C|GetUI_Workbench (Variables|Default|GetUI_Player)) "Collapsed")
    (else
      (Variables|Default|SetbIsOpenedWorkbench true)
      (Variables|Default|SetCharacterStates "E_Interaction")
      (Input|SetInputModeGameandUI _returnvalue _ui_workbench "DoNotLock" false false)
      (Variables|/Script/Engine.PlayerController|SetbShowMouseCursor _returnvalue true)
      (Widget|SetVisibility _ui_workbench "Visible")
      (Default|UpdateItemInfo _ui_workbench))))

(event Custom|UpdateInfo
  ;[1 1 1] 打开工作台UI
  (Default|UpdateItemInfo (Variables|/Game/_Game/UMG/_Player/UI_Player.UI_Player_C|GetUI_Workbench (Variables|Default|GetUI_Player))))

(event EventBeginPlay
  (bind _returnvalue (UserInterface|CreateWidget "/Game/_Game/UMG/_Player/UI_Player.UI_Player_C"))
  (bind _output_get (Variables|Default|SetUI_Player _returnvalue))
  (UserInterface|Viewport|AddtoViewport _output_get 0))

(event EventTick
  (params (DeltaSeconds :type Float%20%28single-precision%29))
  (CallFunction|SpawnTool)
  (CallFunction|OpenBackpack)
  (CallFunction|OpenChangeMesh))

(fn ConstructionScript)

(fn SpawnTool
  (if (Variables|Default|GetbIsSpawnTool)
    (Variables|Default|SetbIsSpawnTool false)
    (LocalVariables|SetSocketTransform (Transformation|GetSocketTransform (Variables|Character|GetMesh) "Tool" "RTS_World"))
    (switch Utilities|FlowControl|Switch|SwitchonEBackpackClass (.class (Utilities|Array|Get(acopy) (Variables|Default|GetShortcutItemInfo) (Variables|Default|GetCurrentShortcutIndex)))
      (:E_Axe
        (Variables|Default|SetToolClass "/Game/_Game/_Player/_Blueprint/Tools/BP_Tools_Axe.BP_Tools_Axe_C"))
      (:E_Pickaxe
        (Variables|Default|SetToolClass "/Game/_Game/_Player/_Blueprint/Tools/BP_Tools_Pickaxe.BP_Tools_Pickaxe_C"))
      (:E_Hammer
        (Variables|Default|SetToolClass "/Game/_Game/_Player/_Blueprint/Tools/BP_Tools_Hammer.BP_Tools_Hammer_C")))
    (bind _returnvalue (Game|SpawnActorfromClass (Variables|Default|GetToolClass) (LocalVariables|GetSocketTransform) "Undefined" "MultiplyWithRoot" 0 0))
    (bind _output_get (Variables|Default|SetToolActor _returnvalue))
    (Transformation|AttachComponentToComponent _output_get (Variables|Character|GetMesh) "Tool" "SnapToTarget" "SnapToTarget" "SnapToTarget" true)))

(fn BackpackAdd
  (params (NewParam :type F%20Backpack%20Info%20Structure))
  (bind _backpackiteminfo (Variables|Default|GetBackpackItemInfo))
  ;[1 1 1] 添加背包物资
  (Variables|Default|SetItemInfo NewParam)
  (if (Utilities|Array|IsNotEmpty (Variables|Default|GetBackpackItemInfo))
    (if (.IsStack (Utilities|Struct|BreakFBackpackInfo (Variables|Default|GetItemInfo)))
      (bind (_array_element _array_index) (Utilities|Array|ForEachLoopwithBreak (Variables|Default|GetBackpackItemInfo) :!label _label)
        (:LoopBody
          (if (Utilities|Enum|Equal(Enum) (.Name (Utilities|Struct|BreakFBackpackInfo (Variables|Default|GetItemInfo))) (.Name (Utilities|Struct|BreakFBackpackInfo _array_element)))
            (if (< (.Count (Utilities|Struct|BreakFBackpackInfo _array_element)) (.MaxCount (Utilities|Struct|BreakFBackpackInfo _array_element)))
              (Utilities|Array|SetArrayElem (Variables|Default|GetBackpackItemInfo) _array_index (Utilities|Struct|MakeFBackpackInfo (.Name (Utilities|Struct|BreakFBackpackInfo (Variables|Default|GetItemInfo))) (.Index (Utilities|Struct|BreakFBackpackInfo _array_element)) (.Image (Utilities|Struct|BreakFBackpackInfo (Variables|Default|GetItemInfo))) (.IsStack (Utilities|Struct|BreakFBackpackInfo (Variables|Default|GetItemInfo))) (+ (.Count (Utilities|Struct|BreakFBackpackInfo _array_element)) (.Count (Utilities|Struct|BreakFBackpackInfo (Variables|Default|GetItemInfo)))) (.MaxCount (Utilities|Struct|BreakFBackpackInfo (Variables|Default|GetItemInfo))) (.Class (Utilities|Struct|BreakFBackpackInfo (Variables|Default|GetItemInfo))) (.IsEmpty (Utilities|Struct|BreakFBackpackInfo (Variables|Default|GetItemInfo))) (.SortNum (Utilities|Struct|BreakFBackpackInfo (Variables|Default|GetItemInfo))) (.CanUse (Utilities|Struct|BreakFBackpackInfo (Variables|Default|GetItemInfo)))))
              (LocalVariables|SetIsNew false)
              (goto _label Break)
              (else
                _)))
          (LocalVariables|SetIsNew true))
        (:Completed
          (if (LocalVariables|GetIsNew)
            (bind _returnvalue (Utilities|Array|Add _backpackiteminfo (Variables|Default|GetItemInfo) :!label _label_2))
            (Utilities|Array|SetArrayElem _backpackiteminfo _returnvalue (Utilities|Struct|MakeFBackpackInfo (.Name (Utilities|Struct|BreakFBackpackInfo (Variables|Default|GetItemInfo))) _returnvalue (.Image (Utilities|Struct|BreakFBackpackInfo (Variables|Default|GetItemInfo))) (.IsStack (Utilities|Struct|BreakFBackpackInfo (Variables|Default|GetItemInfo))) (.Count (Utilities|Struct|BreakFBackpackInfo (Variables|Default|GetItemInfo))) (.MaxCount (Utilities|Struct|BreakFBackpackInfo (Variables|Default|GetItemInfo))) (.Class (Utilities|Struct|BreakFBackpackInfo (Variables|Default|GetItemInfo))) (.IsEmpty (Utilities|Struct|BreakFBackpackInfo (Variables|Default|GetItemInfo))) (.SortNum (Utilities|Struct|BreakFBackpackInfo (Variables|Default|GetItemInfo))) (.CanUse (Utilities|Struct|BreakFBackpackInfo (Variables|Default|GetItemInfo))))))))
      (else
        (goto _label_2)))
    (else
      (goto _label_2))))

(fn OpenBackpack
  (bind _returnvalue (Game|GetPlayerController 0))
  (bind _ui_player (Variables|Default|GetUI_Player))
  (bind _ui_backpack (Variables|/Game/_Game/UMG/_Player/UI_Player.UI_Player_C|GetUI_Backpack _ui_player))
  ;[1 1 1] 打开背包UI
  (if (Variables|Default|GetIsOpenBackpack)
    (Variables|Default|SetIsOpenBackpack false)
    (if (Variables|Default|GetbIsOpenedBackpack)
      (Variables|Default|SetbIsOpenedBackpack false)
      (Variables|Default|SetCharacterStates "E_Common")
      (Input|SetInputModeGameOnly (Game|GetPlayerController 0) false)
      (Variables|/Script/Engine.PlayerController|SetbShowMouseCursor (Game|GetPlayerController 0) false)
      (Widget|SetVisibility _ui_backpack "Collapsed")
      (Utilities|Time|SetGlobalTimeDilation 1.0)
      (else
        (Variables|Default|SetbIsOpenedBackpack true)
        (Variables|Default|SetCharacterStates "E_OpenBackpack")
        (Input|SetInputModeGameandUI _returnvalue _ui_backpack "DoNotLock" false false)
        (Variables|/Script/Engine.PlayerController|SetbShowMouseCursor _returnvalue true)
        (Variables|/Game/_Game/UMG/_Player/Backpack/UI_Backpack.UI_Backpack_C|SetCnt _ui_backpack (Variables|Default|GetBackpackCnt))
        (Widget|SetVisibility _ui_backpack "Visible")
        (Default|UpdateBackpack _ui_backpack)
        (Utilities|Time|SetGlobalTimeDilation 0.0)))))

(fn ReduceBackpackMaterial
  (params (Name :type Text) (Cnt :type Integer))
  ;[1 1 1] 背包UI中的物资减少
  (LocalVariables|SetReduceName Name)
  (LocalVariables|SetReduceCnt Cnt)
  (for (_array_element _array_index) (Variables|Default|GetBackpackItemInfo)
    (if (Utilities|Enum|Equal(Enum) (.Name (Utilities|Struct|BreakFBackpackInfo _array_element)) (LocalVariables|GetReduceName))
      (if (> (- (.Count (Utilities|Struct|BreakFBackpackInfo _array_element)) (LocalVariables|GetReduceCnt)) 0)
        (Utilities|Array|SetArrayElem (Variables|Default|GetBackpackItemInfo) _array_index (Utilities|Struct|MakeFBackpackInfo (.Name (Utilities|Struct|BreakFBackpackInfo _array_element)) (.Index (Utilities|Struct|BreakFBackpackInfo _array_element)) (.Image (Utilities|Struct|BreakFBackpackInfo _array_element)) (.IsStack (Utilities|Struct|BreakFBackpackInfo _array_element)) (- (.Count (Utilities|Struct|BreakFBackpackInfo _array_element)) (LocalVariables|GetReduceCnt)) (.MaxCount (Utilities|Struct|BreakFBackpackInfo _array_element)) (.Class (Utilities|Struct|BreakFBackpackInfo _array_element)) (.IsEmpty (Utilities|Struct|BreakFBackpackInfo _array_element)) (.SortNum (Utilities|Struct|BreakFBackpackInfo _array_element)) (.CanUse (Utilities|Struct|BreakFBackpackInfo _array_element))))
        (else
          (return _array_index)))))
  (return -1))

(fn ChangeBackpack
  (params (Name :type Text) (Cnt :type Integer) (String :type String))
  ;[1 1 1] 背包物资发生改变
  (Class|GJCharacter|ReduceMaterials String Cnt)
  (bind _removeindex (CallFunction|ReduceBackpackMaterial Name Cnt))
  (if (!= _removeindex -1)
    (CallFunction|DeleteBackpackInfo _removeindex)
    (else
      (Default|UpdateBackpack (Variables|/Game/_Game/UMG/_Player/UI_Player.UI_Player_C|GetUI_Backpack (Variables|Default|GetUI_Player))))))

(fn SwapBackpackItem
  (params (SecondIndex :type Integer) (SecondParent :type String))
  (bind _ui_player (Variables|Default|GetUI_Player))
  (bind _shortcutiteminfo (Variables|Default|GetShortcutItemInfo))
  (bind _switchstarttarget (Variables|Default|GetSwitchStartTarget))
  (bind _backpackiteminfo (Variables|Default|GetBackpackItemInfo))
  (bind _output (Utilities|Array|Get(acopy) _shortcutiteminfo _switchstarttarget))
  (bind (_name _index _image _isstack _count _maxcount _class _isempty _sortnum _canuse) (Utilities|Struct|BreakFBackpackInfo _output))
  (LocalVariables|SetSecond SecondIndex)
  (switch string (Variables|Default|GetSwitchStartTargetParent)
    (:GridPanel
      (switch string SecondParent
        (:GridPanel
          ;[1 1 1] 交换背包物资
          (if (!= (LocalVariables|GetSecond) -1)
            (Utilities|Array|Swap (Variables|Default|GetBackpackItemInfo) (Variables|Default|GetSwitchStartTarget) (LocalVariables|GetSecond))
            (Default|UpdateShortcut (Variables|/Game/_Game/UMG/_Player/UI_Player.UI_Player_C|GetUI_Shortcut _ui_player) :!label _label)
            (Default|UpdateBackpack (Variables|/Game/_Game/UMG/_Player/UI_Player.UI_Player_C|GetUI_Backpack _ui_player))))
        (:Shortcut
          ;[1 1 1] 从背包拖到快捷菜单
          (if (.canuse (Utilities|Array|Get(acopy) (Variables|Default|GetBackpackItemInfo) (Variables|Default|GetSwitchStartTarget)))
            (if (.isempty (Utilities|Array|Get(acopy) (Variables|Default|GetShortcutItemInfo) (LocalVariables|GetSecond)))
              (Utilities|Array|SetArrayElem (Variables|Default|GetShortcutItemInfo) (LocalVariables|GetSecond) (Utilities|Array|Get(acopy) (Variables|Default|GetBackpackItemInfo) (Variables|Default|GetSwitchStartTarget)))
              (CallFunction|DeleteBackpackInfo (Variables|Default|GetSwitchStartTarget))
              (else
                (LocalVariables|SetTempInfo (Utilities|Array|Get(acopy) (Variables|Default|GetShortcutItemInfo) (LocalVariables|GetSecond)))
                (Utilities|Array|SetArrayElem (Variables|Default|GetShortcutItemInfo) (LocalVariables|GetSecond) (Utilities|Array|Get(acopy) (Variables|Default|GetBackpackItemInfo) (Variables|Default|GetSwitchStartTarget)))
                (Utilities|Array|SetArrayElem (Variables|Default|GetBackpackItemInfo) (Variables|Default|GetSwitchStartTarget) (LocalVariables|GetTempInfo))))
            (Utilities|Array|SetArrayElem (Variables|Default|GetShortcutIsEmpty) (LocalVariables|GetSecond) false)
            (goto _label)))))
    (:Shortcut
      (switch string SecondParent
        (:GridPanel
          ;[1 1 1] 从快捷菜单拖到背包
          (if (!= (LocalVariables|GetSecond) -1)
            (LocalVariables|SetTempInfo (Utilities|Array|Get(acopy) (Variables|Default|GetBackpackItemInfo) (LocalVariables|GetSecond)))
            (Utilities|Array|SetArrayElem (Variables|Default|GetBackpackItemInfo) (LocalVariables|GetSecond) (Utilities|Array|Get(acopy) (Variables|Default|GetShortcutItemInfo) (Variables|Default|GetSwitchStartTarget)))
            (Utilities|Array|SetArrayElem (Variables|Default|GetShortcutItemInfo) (Variables|Default|GetSwitchStartTarget) (LocalVariables|GetTempInfo))
            (goto _label)
            (else
              (bind _returnvalue (Utilities|Array|Add _backpackiteminfo _output))
              (Utilities|Array|SetArrayElem _backpackiteminfo _returnvalue (Utilities|Struct|MakeFBackpackInfo _name _returnvalue _image _isstack _count _maxcount _class _isempty _sortnum _canuse))
              (Utilities|Array|SetArrayElem (Variables|Default|GetShortcutItemInfo) (Variables|Default|GetSwitchStartTarget) (LocalVariables|GetEmpty))
              (Utilities|Array|SetArrayElem (Variables|Default|GetShortcutIsEmpty) (Variables|Default|GetSwitchStartTarget) false)
              (goto _label))))
        (:Shortcut
          ;[1 1 1] 快捷菜单之间交换
          (Utilities|Array|Swap (Variables|Default|GetShortcutItemInfo) (Variables|Default|GetSwitchStartTarget) (LocalVariables|GetSecond))
          (Utilities|Array|SetArrayElem (Variables|Default|GetShortcutIsEmpty) (LocalVariables|GetSecond) false)
          (Utilities|Array|SetArrayElem (Variables|Default|GetShortcutIsEmpty) (Variables|Default|GetSwitchStartTarget) (== (LocalVariables|GetSecond) 0))
          (goto _label))))))

(fn DeleteBackpackInfo
  (params (IndexToRemove :type Integer))
  ;[1 1 1] 删除背包资源
  (Utilities|Array|RemoveIndex (Variables|Default|GetBackpackItemInfo) IndexToRemove)
  (for (_array_element _array_index) (Variables|Default|GetBackpackItemInfo)
    (Utilities|Array|SetArrayElem (Variables|Default|GetBackpackItemInfo) _array_index (Utilities|Struct|MakeFBackpackInfo (.Name (Utilities|Struct|BreakFBackpackInfo _array_element)) _array_index (.Image (Utilities|Struct|BreakFBackpackInfo _array_element)) (.IsStack (Utilities|Struct|BreakFBackpackInfo _array_element)) (.Count (Utilities|Struct|BreakFBackpackInfo _array_element)) (.MaxCount (Utilities|Struct|BreakFBackpackInfo _array_element)) (.Class (Utilities|Struct|BreakFBackpackInfo _array_element)) (.IsEmpty (Utilities|Struct|BreakFBackpackInfo _array_element)) (.SortNum (Utilities|Struct|BreakFBackpackInfo _array_element)) (.CanUse (Utilities|Struct|BreakFBackpackInfo _array_element)))))
  (Default|UpdateBackpack (Variables|/Game/_Game/UMG/_Player/UI_Player.UI_Player_C|GetUI_Backpack (Variables|Default|GetUI_Player))))

(fn OpenChangeMesh
  (bind _returnvalue (Game|GetPlayerController 0))
  (bind _ui_player (Variables|Default|GetUI_Player))
  (bind _ui_changemesh (Variables|/Game/_Game/UMG/_Player/UI_Player.UI_Player_C|GetUI_ChangeMesh _ui_player))
  ;[1 1 1] 打开背包UI
  (if (Variables|Default|GetIsOpenChangeMesh)
    (Variables|Default|SetIsOpenChangeMesh false)
    (if (Variables|Default|GetIsOpenedChangeMesh)
      (Variables|Default|SetIsOpenedChangeMesh false)
      (Variables|Default|SetCharacterStates "E_Common")
      (Input|SetInputModeGameOnly (Game|GetPlayerController 0) false)
      (Variables|/Script/Engine.PlayerController|SetbShowMouseCursor (Game|GetPlayerController 0) false)
      (Widget|SetVisibility _ui_changemesh "Collapsed")
      (Utilities|Time|SetGlobalTimeDilation 1.0)
      (else
        (Variables|Default|SetIsOpenedChangeMesh true)
        (Variables|Default|SetCharacterStates "E_OpenChangeMesh")
        (Input|SetInputModeGameandUI _returnvalue 0 "DoNotLock" false false)
        (Variables|/Script/Engine.PlayerController|SetbShowMouseCursor _returnvalue true)
        (Widget|SetVisibility _ui_changemesh "Visible")
        (Default|UpdateInfo _ui_changemesh)
        (Utilities|Time|SetGlobalTimeDilation 0.0)))))